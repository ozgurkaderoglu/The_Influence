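; BP_DI_Carpenter is the Carpenter player character for The Island, with debug-style key bindings for a gate and subtitles.
; On BeginPlay it creates the WGP_Ui widget and adds it to the viewport.
; Key 1 finds the level's Gate_BP and, when it is not in use, alternates between starting and returning it.
; Key 2 passes itself to BPSubtitles, and the StartSubtitles event pushes the current subtitle line to the widget.
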(event EventBeginPlay
  (bind _returnvalue (UserInterface|CreateWidget "/Game/NewGameplayBuild/UI/WGP_Ui.WGP_Ui_C"))
  (bind _output_get (Variables|PlayerUI|SetWGP_UI _returnvalue))
  (UserInterface|Viewport|AddtoViewport _output_get 0))

(event Input|KeyboardEvents|2
  (params (Key :type Key%20Structure :default "None"))
  (:Pressed
    (Default|StartSubtitle (Variables|Default|GetBP_Subtitles) self)))

(event Input|KeyboardEvents|1
  (params (Key :type Key%20Structure :default "None"))
  (:Pressed
    (bind _returnvalue (Actor|GetActorOfClass "/Game/_Level/_Blueprints/Gate_BP.Gate_BP_C"))
    (if (Variables|/Game/_Level/_Blueprints/Gate_BP.Gate_BP_C|GetIsGateNotInUse? _returnvalue)
      (Utilities|FlowControl|FlipFlop
        (:A
          (Default|StartGate _returnvalue))
        (:B
          (Default|ReturnGate _returnvalue))))))

(event Custom|Start%20Subtitles
  (Default|SetNewSibtitleLine (Variables|PlayerUI|GetWGP_UI) (Utilities|Text|ToText(String) (Variables|/Game/_SubtitleSystem/BP_Subtitles.BP_Subtitles_C|GetSubtitle%20To%20Widget (Variables|Default|GetBP_Subtitles)))))

(fn ConstructionScript)