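; BP_Subtitles plays a timed sequence of subtitle lines through the player character, supporting both BP_DI_Carpenter and BP_DI_CarpNew.
; StartSubtitle stores the current line in SubtitleToWidget, debug-prints it and calls StartSubtitles on the player.
; After that line's own delay and a short gap, StartNextLine loops back until MaxSubtitleLines is reached.
; The line index is never reset in this graph.
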(event Custom|Start%20Subtitle
  (params (Player :type Actor%20Object%20Reference))
  (bind _asbp_di_carpenter (Utilities|Casting|CastToBP_DI_Carpenter Player)
    (:then
      _)
    (:CastFailed
      (bind _asbp_di_carp_new (Utilities|Casting|CastToBP_DI_CarpNew Player))))
  (Development|PrintString (Utilities|Array|Get(acopy) (Variables|Default|GetSubtitle%20Lines) (Variables|Default|GetLine%20OF%20Subtitles)))
  (Variables|Default|SetSubtitle%20To%20Widget (Utilities|Array|Get(acopy) (Variables|Default|GetSubtitle%20Lines) (Variables|Default|GetLine%20OF%20Subtitles)))
  (Utilities|IsValid _asbp_di_carpenter
    (:Is%20Valid
      (Default|StartSubtitles _asbp_di_carpenter))
    (:Is%20Not%20Valid
      (Default|StartSubtitles _asbp_di_carp_new)))
  (Utilities|FlowControl|Delay (Utilities|Array|Get(acopy) (Variables|Default|GetTime%20Between%20Lines) (Variables|Default|GetLine%20OF%20Subtitles)))
  (Variables|Default|SetLine%20OF%20Subtitles (+ (Variables|Default|GetLine%20OF%20Subtitles) 1))
  (Utilities|FlowControl|Delay 0.2)
  (CallFunction|StartNextLine))

(event Custom|Start%20NextLine
  (if (not (> (Variables|Default|GetLine%20OF%20Subtitles) (- (Variables|Default|GetMax%20Subtitle%20Lines) 1)))
    (Development|PrintString (Utilities|Array|Get(acopy) (Variables|Default|GetSubtitle%20Lines) (Variables|Default|GetLine%20OF%20Subtitles)))
    (Variables|Default|SetSubtitle%20To%20Widget (Utilities|Array|Get(acopy) (Variables|Default|GetSubtitle%20Lines) (Variables|Default|GetLine%20OF%20Subtitles)))
    (Utilities|IsValid (stale Custom|Start%20Subtitle _asbp_di_carpenter)
      (:Is%20Valid
        (Default|StartSubtitles (stale Custom|Start%20Subtitle _asbp_di_carpenter)))
      (:Is%20Not%20Valid
        (Default|StartSubtitles (stale Custom|Start%20Subtitle _asbp_di_carp_new))))
    (Utilities|FlowControl|Delay (Utilities|Array|Get(acopy) (Variables|Default|GetTime%20Between%20Lines) (Variables|Default|GetLine%20OF%20Subtitles)))
    (Variables|Default|SetLine%20OF%20Subtitles (+ (Variables|Default|GetLine%20OF%20Subtitles) 1))
    (Utilities|FlowControl|Delay 0.2)
    (CallFunction|StartNextLine)))

(event EventBeginPlay)

(event EventTick
  (params (DeltaSeconds :type Float%20%28single-precision%29)))