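; Player character Blueprint that handles face animation, cutscene no-clip, camera reset and startup display settings.
; Random-interval blinks and voice-envelope mouth movement write to mesh custom primitive data to drive the face.
; BeginPlay starts the blink loop and forces fullscreen, 25% screen percentage and a 30 FPS cap through console commands.
; Tank movement, jumping and mouse-orbit camera logic with idle reset is present but has no triggering events connected.
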(event OnAudioMultiEnvelopeValue(Speech_Voice)
  (params (AverageEnvelopeValue :type Float%20%28single-precision%29) (MaxEnvelope :type Float%20%28single-precision%29) (NumWaveInstances :type Integer))
  ;[1 1 1] Enable Speech Movement
  (bind _output_get (Variables|Default|SetSpeech_Amount (* AverageEnvelopeValue (Variables|Default|GetVoice_Sensitivity))))
  (Rendering|Material|SetCustomPrimitiveDataFloat (Variables|Character|GetMesh) 31 _output_get))

(event Custom|Stop_Mouth
  ;[1 1 1] Enable Speech Movement
  (bind _output_get (Variables|Default|SetSpeech_Amount 0.0))
  (Rendering|Material|SetCustomPrimitiveDataFloat (Variables|Character|GetMesh) 31 _output_get))

(event Custom|Reset_Camera
  ;[1 1 1] Mouse Control
  ;;[1 1 1] Reset camera after an amount of time
  (Transformation|SetRelativeRotation (Variables|MyCharacter|GetCameraBoom) (Math|Rotator|MakeRotator 0.0 0.0 (.yaw (Transformation|GetWorldRotation (Variables|Collision|GetCapsuleComponent)))) false false))

(event Custom|Event_No_Clip_Enabled
  ;[1 1 1] No clipping for cutscenes where collision would cause issues
  (Collision|SetCollisionEnabled (Variables|Collision|GetCapsuleComponent) "NoCollision")
  (Pawn|Components|CharacterMovement|SetMovementMode (Variables|Character|GetCharacterMovement) "MOVE_None" 0)
  (Variables|Default|SetNo_Clip_Enabled? true))

(event Custom|Event_No_Clip_Disabled
  ;[1 1 1] No clipping for cutscenes where collision would cause issues
  (Collision|SetCollisionEnabled (Variables|Collision|GetCapsuleComponent) "QueryAndPhysics")
  (Pawn|Components|CharacterMovement|SetMovementMode (Variables|Character|GetCharacterMovement) "MOVE_Walking" 0)
  (Variables|Default|SetNo_Clip_Enabled? false))

(event Custom|Blink
  (bind _mesh (Variables|Character|GetMesh))
  ;[1 1 1] Blinking
  (Utilities|FlowControl|Sequence :!label _label
    (:then_0
      (Utilities|FlowControl|RetriggerableDelay (Math|Random|RandomFloatinRange 1.0 3.0))
      (goto _label))
    (:then_1
      (bind _output_get (Variables|Default|SetBlink_Value 1.0))
      (Rendering|Material|SetCustomPrimitiveDataFloat _mesh 30 _output_get)
      (Utilities|FlowControl|Delay 0.2)
      (bind _output_get_2 (Variables|Default|SetBlink_Value 0.0))
      (Rendering|Material|SetCustomPrimitiveDataFloat _mesh 30 _output_get_2))))

(event EventBeginPlay
  ;[1 1 1] BeginPlay
  ;[1 1 1] Calling blink event
  (CallFunction|Blink)
  ;[1 1 1] Setting Game Settings
  (|Game_Settings))

(fn ConstructionScript)