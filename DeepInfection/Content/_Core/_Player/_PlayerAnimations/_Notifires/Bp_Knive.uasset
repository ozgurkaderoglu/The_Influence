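; Animation notify in the player animations folder that applies a knife stab's melee damage to enemies.
; When it fires, it sphere-traces a short distance forward from the mesh owner on the Visibility channel, with debug drawing on.
; If the hit actor is an Enemy_Main, it applies fixed damage and plays the stab sound at the world origin rather than the hit point.
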(fn ReceivedNotify
  (params (MeshComp :type Skeletal%20Mesh%20Component%20Object%20Reference) (Animation :type Anim%20Sequence%20Base%20Object%20Reference) (EventReference :type Anim%20Notify%20Event%20Reference%20Structure%20%28by%20ref%29))
  (bind _returnvalue (Components|GetOwner MeshComp))
  (bind _returnvalue_2 (Transformation|GetActorLocation _returnvalue))
  (bind (_outhit _returnvalue_3) (Collision|SphereTraceByChannel _returnvalue_2 (+ _returnvalue_2 (* (Transformation|GetActorForwardVector _returnvalue) 1e+02)) 2e+01 "TraceTypeQuery1" false 0 "ForDuration"))
  (if _returnvalue_3
    (bind _asenemy_main (Utilities|Casting|CastToEnemy_Main (.HitActor (Collision|BreakHitResult _outhit))))
    (Game|Damage|ApplyDamage _asenemy_main 9e+01 0 0)
    (Audio|PlaySoundatLocation "/Game/_Core/Item_sounds/Knife_Stab.Knife_Stab" "0, 0, 0" "0, 0, 0" 1.0 1.0 0.0 0 0 0 0)))