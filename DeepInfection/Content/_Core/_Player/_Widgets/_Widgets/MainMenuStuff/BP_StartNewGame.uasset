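; Main menu trigger actor that starts a new game or continues a saved one when the DI_Player overlaps its static mesh.
; The Continuegame flag picks the mode, and the construction script sets the text label to match.
; On overlap it moves the player to their SavedLocation or to the StartLocation component, clears InMainMenu and calls BeginPlayGameplay.
; The Box overlap event is empty.
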(event OnComponentBeginOverlap(Box)
  (params (OverlappedComponent :type Primitive%20Component%20Object%20Reference) (OtherActor :type Actor%20Object%20Reference) (OtherComp :type Primitive%20Component%20Object%20Reference) (OtherBodyIndex :type Integer) (bFromSweep :type Boolean) (SweepResult :type Hit%20Result%20Structure%20%28by%20ref%29)))

(event OnComponentBeginOverlap(StaticMesh)
  (params (OverlappedComponent :type Primitive%20Component%20Object%20Reference) (OtherActor :type Actor%20Object%20Reference) (OtherComp :type Primitive%20Component%20Object%20Reference) (OtherBodyIndex :type Integer) (bFromSweep :type Boolean) (SweepResult :type Hit%20Result%20Structure%20%28by%20ref%29))
  (if (Variables|Default|GetContinuegame)
    (if true
      (bind _asdi_player (Utilities|Casting|CastToDI_Player OtherActor))
      (Transformation|SetActorLocation _asdi_player (Variables|/Game/_Core/_Player/DI_Player.DI_Player_C|GetSavedLocation _asdi_player) false false)
      (Variables|/Game/_Core/_Player/DI_Player.DI_Player_C|SetIn%20Main%20menu _asdi_player false)
      (Default|BeginPlayGameplay _asdi_player))
    (else
      (bind _asdi_player_2 (Utilities|Casting|CastToDI_Player OtherActor))
      (Transformation|SetActorLocation _asdi_player_2 (Transformation|GetWorldLocation (Variables|Default|GetStart%20Location)) false false)
      (Variables|/Game/_Core/_Player/DI_Player.DI_Player_C|SetIn%20Main%20menu _asdi_player_2 false)
      (Default|BeginPlayGameplay _asdi_player_2))))

(event EventBeginPlay)

(event Collision|EventActorBeginOverlap
  (params (OtherActor :type Actor%20Object%20Reference)))

(event EventTick
  (params (DeltaSeconds :type Float%20%28single-precision%29)))

(fn ConstructionScript
  (if (Variables|Default|GetContinuegame)
    (Rendering|Components|TextRender|SetText (Variables|Default|GetTextRender) (Utilities|Text|MakeLiteralText "CONTINUE GAME"))
    (else
      (Rendering|Components|TextRender|SetText (Variables|Default|GetTextRender) (Utilities|Text|MakeLiteralText "New game")))))