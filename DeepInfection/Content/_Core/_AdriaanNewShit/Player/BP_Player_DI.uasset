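; Player Blueprint that handles directional movement, captain interaction, UI and the cutscene save game.
; BeginPlay creates or loads the save, restoring position when LoadedPlay is set; StartNewGame writes the start location and opens the cutscene level.
; N/E/S/W flags remap Enhanced Input axes to suit the current direction.
; Interaction pauses movement while timelines lerp the cine camera and toggle the captain widget; keys also toggle a console and delete the save.
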(event Custom|Start%20New%20Game
  (bind _cutcenesaveref (Variables|Default|GetCutceneSaveRef))
  (bind _returnvalue (SaveGame|DoesSaveGameExist "1")) ; 1 = cutcene
  (if _returnvalue
    (Variables|/Game/_Core/_AdriaanNewShit/SaveSystems/CutceneSaveSystem/BP_CutceneSave_DI.BP_CutceneSave_DI_C|SetNewGame _cutcenesaveref true)
    (Variables|/Game/_Core/_AdriaanNewShit/SaveSystems/CutceneSaveSystem/BP_CutceneSave_DI.BP_CutceneSave_DI_C|SetLocation _cutcenesaveref (Variables|Default|GetNewGameStart))
    (Variables|/Game/_Core/_AdriaanNewShit/SaveSystems/CutceneSaveSystem/BP_CutceneSave_DI.BP_CutceneSave_DI_C|SetLoadedPlay? _cutcenesaveref true)
    (bind _returnvalue_2 (SaveGame|SaveGametoSlot _cutcenesaveref "1"))
    (if _returnvalue_2
      (Game|OpenLevel(byObjectReference) "/Game/_Level/Cutscenes.Cutscenes"))))

(event Custom|Start%20Loaded%20Game)

(event Custom|Open%20Level%20With%20NewGame)

(event Custom|LoadGame
  (CallFunction|LoadingGame)
  (Variables|Default|SetPlayOnLoadGame true))

(event Custom|SetNEwGameLocation
  (params (NewGameStart :type Vector))
  (Variables|Default|SetNewGameStart NewGameStart))

(event Custom|SetBackPlayOnLoadgame
  (bind _cutcenesaveref (Variables|Default|GetCutceneSaveRef))
  (if (Variables|Default|GetPlayOnLoadGame)
    (Utilities|FlowControl|Delay 3e+01)
    (bind _output_get (Variables|Default|SetPlayOnLoadGame false))
    (Variables|/Game/_Core/_AdriaanNewShit/SaveSystems/CutceneSaveSystem/BP_CutceneSave_DI.BP_CutceneSave_DI_C|SetLoadedPlay? _cutcenesaveref _output_get)
    (bind _returnvalue (SaveGame|DoesSaveGameExist "1")) ; 1 = cutcene
    (if _returnvalue
      (bind _returnvalue_2 (SaveGame|SaveGametoSlot _cutcenesaveref "1"))
      (if _returnvalue_2
        (Development|PrintString "Settingback olay on loaded")))))

(event EventBeginPlay
  (CallFunction|CreateAllWidgeds)
  (bind _returnvalue (SaveGame|DoesSaveGameExist "1")) ; 1 = cutcene
  (if _returnvalue
    (bind _returnvalue_2 (SaveGame|LoadGamefromSlot "1"))
    (bind _asbp_cutcene_save_di (Utilities|Casting|CastToBP_CutceneSave_DI _returnvalue_2))
    (Variables|Default|SetCutceneSaveRef _asbp_cutcene_save_di)
    (CallFunction|LoadingGame)
    (CallFunction|SetBackPlayonLoadgame)
    (else
      (bind _returnvalue_3 (SaveGame|CreateSaveGameObject "/Game/_Core/_AdriaanNewShit/SaveSystems/CutceneSaveSystem/BP_CutceneSave_DI.BP_CutceneSave_DI_C"))
      (bind _output_get (Variables|Default|SetCutceneSaveRef _returnvalue_3))
      (SaveGame|SaveGametoSlot _output_get "1"))))

(event Input|KeyboardEvents|2
  (params (Key :type Key%20Structure :default "None")))

(event Input|KeyboardEvents|1
  (params (Key :type Key%20Structure :default "None"))
  (:Pressed
    (SaveGame|DeleteGameinSlot "1")))

(event Custom|Open_Console
  (bind _returnvalue (UserInterface|CreateWidget "/Game/FInalGameBuild/Widgets/Console/WGP_DI_Console.WGP_DI_Console_C"))
  (bind _output_get (Variables|PlayerUI|SetDi_Console _returnvalue))
  (UserInterface|Viewport|AddtoViewport _output_get 0))

(event Custom|Close_Console
  (Widget|SetVisibility (Variables|PlayerUI|GetDi_Console) "Collapsed"))

(event Custom|Create%20All%20Widgeds
  (Utilities|FlowControl|Sequence
    (:then_0
      (bind _returnvalue (UserInterface|CreateWidget "/Game/_Core/_AdriaanNewShit/Widgets/Captain/WBP_Captain_Di.WBP_Captain_Di_C"))
      (bind _output_get (Variables|Widgets|SetWBP_Cap _returnvalue))
      (UserInterface|Viewport|AddtoViewport _output_get 0)
      (Widget|SetVisibility _output_get "Collapsed"))))

(event Custom|Get%20Info%20From%20cap
  (params (Target :type Object%20Object%20Reference))
  (Variables|Captain/Ferryman|SetCap Target))

(event Custom|Reset%20Do%20Once%20Cap
  (Utilities|FlowControl|DoOnce false) ; enters at Reset
)

(event Input|EnhancedActionEvents|EnhancedInputActionIA_Move
  (params (ActionValue :type Vector%202D%20Structure) (ElapsedSeconds :type Float%20%28double-precision%29) (TriggeredSeconds :type Float%20%28double-precision%29) (InputAction :type Input%20Action%20Object%20Reference :default "/Game/_Core/_Player/_Inputs/_IA/IA_Move.IA_Move"))
  (if (not (Variables|Camera|GetPause%20Movement))
    (if (Variables|PlayerUI|GetN)
      (CallFunction|Movement (.x ActionValue) (.y ActionValue))
      (elif (Variables|PlayerUI|GetE)
        (bind _result (Math|Float|NegateFloat (.x ActionValue))
          (:%20%20
            (CallFunction|Movement (.y ActionValue) _result)))
        (elif (Variables|PlayerUI|GetS)
          (bind _result_2 (Math|Float|NegateFloat (.x ActionValue))
            (:%20%20
              (bind _result_3 (Math|Float|NegateFloat (.y ActionValue))
                (:%20%20
                  (CallFunction|Movement _result_2 _result_3)))))
          (elif (Variables|PlayerUI|GetW)
            (bind _result_4 (Math|Float|NegateFloat (.y ActionValue))
              (:%20%20
                (CallFunction|Movement _result_4 (.x ActionValue))))))))))

(event Input|KeyboardEvents|RightBracket
  (params (Key :type Key%20Structure))
  (bind _returnvalue (Game|GetPlayerController 0))
  (:Pressed
    (Utilities|FlowControl|FlipFlop
      (:A
        (CallFunction|OpenConsole)
        (Variables|/Script/Engine.PlayerController|SetbShowMouseCursor _returnvalue true))
      (:B
        (CallFunction|CloseConsole)
        (Variables|/Script/Engine.PlayerController|SetbShowMouseCursor _returnvalue false)))))

(event Input|KeyboardEvents|E
  (params (Key :type Key%20Structure))
  (:Pressed
    (if (Variables|Captain/Ferryman|GetCan%20Interact%20with%20Cap)
      (Utilities|FlowControl|DoOnce false
        (:Completed
          (Utilities|FlowControl|FlipFlop
            (:A
              (Class|BPICapDI|StartCamS(Message) (Variables|Captain/Ferryman|GetCap) false))
            (:B
              (CallFunction|ResetBacktoBasic))))))))

(event Custom|Start%20New%20Camera%20Pos
  (params (New%20CameraLocation :type Vector) (New%20Camera%20Rotat :type Rotator))
  (bind _cinecamera_temp (Variables|Default|GetCineCamera%20TEMP))
  (Variables|Camera|SetPause%20Movement true)
  (Variables|Camera|SetNew%20Camera%20Rotat New%20Camera%20Rotat)
  (Variables|Camera|SetNew%20CameraLocation New%20CameraLocation)
  (Variables|Camera|SetBase%20Location (Transformation|GetWorldLocation (Variables|Default|GetCineCamera%20TEMP)))
  (Variables|Camera|SetBase%20Camera%20Rot (Transformation|GetWorldRotation (Variables|Default|GetCineCamera%20TEMP)))
  (bind _cameramovement (Timeline|Timeline PlayFromStart)
    (:Update
      (Transformation|SetWorldLocation _cinecamera_temp (Math|Vector|Lerp(Vector) (Variables|Camera|GetBase%20Location) (Variables|Camera|GetNew%20CameraLocation) _cameramovement) false false)
      (Transformation|SetWorldRotation _cinecamera_temp (Math|Rotator|Lerp(Rotator) (Variables|Camera|GetBase%20Camera%20Rot) (Variables|Camera|GetNew%20Camera%20Rotat) _cameramovement) false false))
    (:Finished
      (CallFunction|ResetDoOnceCap)
      (if (Variables|Captain/Ferryman|GetCan%20Interact%20with%20Cap)
        (Widget|SetVisibility (Variables|Widgets|GetWBP_Cap) "Visible")
        (CallFunction|FocusonUI true)))))

(event Custom|Reset%20back%20To%20Basic
  (bind _cinecamera_temp (Variables|Default|GetCineCamera%20TEMP))
  (Utilities|FlowControl|Sequence
    (:then_0
      (Widget|SetVisibility (Variables|Widgets|GetWBP_Cap) "Collapsed")
      (bind _cameramovement (Timeline|Timeline_0 PlayFromStart)
        (:Update
          (Transformation|SetWorldLocation _cinecamera_temp (Math|Vector|Lerp(Vector) (Variables|Camera|GetNew%20CameraLocation) (Variables|Camera|GetBase%20Location) _cameramovement) false false)
          (Transformation|SetWorldRotation _cinecamera_temp (Math|Rotator|Lerp(Rotator) (Variables|Camera|GetNew%20Camera%20Rotat) (Variables|Camera|GetBase%20Camera%20Rot) _cameramovement) false false))
        (:Finished
          (Variables|Camera|SetPause%20Movement false)
          (CallFunction|ResetDoOnceCap))))
    (:then_1
      (CallFunction|FocusonUI false))))

(fn ConstructionScript)

(fn Movement
  (params (X :type Float%20%28single-precision%29) (Y :type Float%20%28single-precision%29))
  (bind _returnvalue (Pawn|GetControlRotation :!class /Script/Engine.Pawn))
  (Pawn|Input|AddMovementInput (Math|Vector|GetRightVector (Math|Rotator|MakeRotator (.roll _returnvalue) 0.0 (.yaw _returnvalue))) X false)
  (Pawn|Input|AddMovementInput (Math|Vector|GetForwardVector (Math|Rotator|MakeRotator 0.0 0.0 (.yaw (Pawn|GetControlRotation :!class /Script/Engine.Pawn)))) Y false))

(fn SetMovementDirection
  (params (N :type Boolean) (E :type Boolean) (S :type Boolean) (W :type Boolean))
  (Variables|PlayerUI|SetN N)
  (Variables|PlayerUI|SetE E)
  (Variables|PlayerUI|SetS S)
  (Variables|PlayerUI|SetW W))

(fn FocusonUI
  (params (Show%20Mouse%20Cursor :type Boolean))
  (Variables|/Script/Engine.PlayerController|SetbShowMouseCursor (Game|GetPlayerController 0) Show%20Mouse%20Cursor))

(fn CutcenSelecter
  (params (NewGameCutCene :type Boolean) (NewParam1 :type Boolean) (NewParam2 :type Boolean) (NewParam3 :type Boolean) (NewParam4 :type Boolean) (NewParam5 :type Boolean) (NewParam6 :type Boolean)))

(fn LoadingGame
  (Variables|Default|SetPlayOnLoadGame (Variables|/Game/_Core/_AdriaanNewShit/SaveSystems/CutceneSaveSystem/BP_CutceneSave_DI.BP_CutceneSave_DI_C|GetLoadedPlay? (Variables|Default|GetCutceneSaveRef)))
  (if (not (Variables|Default|GetPlayOnLoadGame))
    (Development|PrintString "Play on  Main menu ")
    (else
      (Transformation|SetActorLocation (Variables|/Game/_Core/_AdriaanNewShit/SaveSystems/CutceneSaveSystem/BP_CutceneSave_DI.BP_CutceneSave_DI_C|GetLocation (Variables|Default|GetCutceneSaveRef)) false false))))

(fn SaveGame)