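; Game instance that owns the game's BP_CutceneSave_DI save object and loads it synchronously on Init.
; Loadgame reads the slot sync or async, or creates a new save object if none exists; SaveGame writes the cached object back either way.
; Only a successful async load calls CallGameLoaded.
; GetGameData has an empty return in this graph.
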(event EventInit
  (CallFunction|Loadgame false))

(event EventLoadgame
  (params (ASync :type Boolean))
  (bind _returnvalue (SaveGame|DoesSaveGameExist (Variables|Default|GetSlot%20Name)))
  (if _returnvalue
    (if ASync
      (bind _savegame (|AsyncLoadGamefromSlot (Variables|Default|GetSlot%20Name))
        (:then
          (bind _asbp_cutcene_save_di (Utilities|Casting|CastToBP_CutceneSave_DI _savegame))
          (Variables|Default|SetAs%20BP%20Cutcene%20Save%20DI _asbp_cutcene_save_di)
          (Default|CallGameLoaded)))
      (else
        (bind _returnvalue_2 (SaveGame|LoadGamefromSlot (Variables|Default|GetSlot%20Name)))
        (bind _asbp_cutcene_save_di_2 (Utilities|Casting|CastToBP_CutceneSave_DI _returnvalue_2))
        (Variables|Default|SetAs%20BP%20Cutcene%20Save%20DI _asbp_cutcene_save_di_2)))
    (else
      (bind _returnvalue_3 (SaveGame|CreateSaveGameObject "/Game/_Core/_AdriaanNewShit/SaveSystems/CutceneSaveSystem/BP_CutceneSave_DI.BP_CutceneSave_DI_C"))
      (Variables|Default|SetAs%20BP%20Cutcene%20Save%20DI _returnvalue_3))))

(event EventSaveGame
  (params (ASync :type Boolean))
  (bind _slot_name (Variables|Default|GetSlot%20Name))
  (if ASync
    (|AsyncSaveGametoSlot (Variables|Default|GetAs%20BP%20Cutcene%20Save%20DI) _slot_name)
    (else
      (SaveGame|SaveGametoSlot (Variables|Default|GetAs%20BP%20Cutcene%20Save%20DI) _slot_name))))

(fn GetGameData
  (return 0))