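; BP_Captail_DI is an interactable Captain actor that shows a "Press E" prompt when the player enters its sphere.
; Overlap toggles the player's interaction flag and the prompt, and passes the captain to the player.
; While the player is in range, Tick yaws the actor toward the player's capsule and the prompt toward the player's camera.
; StartCamS sends the player a new camera position and rotation from a placed component.
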(event OnComponentBeginOverlap(Sphere)
  (params (OverlappedComponent :type Primitive%20Component%20Object%20Reference) (OtherActor :type Actor%20Object%20Reference) (OtherComp :type Primitive%20Component%20Object%20Reference) (OtherBodyIndex :type Integer) (bFromSweep :type Boolean) (SweepResult :type Hit%20Result%20Structure%20%28by%20ref%29))
  (bind _asbp_player_di (Utilities|Casting|CastToBP_Player_DI OtherActor))
  (bind _output_get (Variables|Default|SetAs%20BP%20Player%20DI _asbp_player_di))
  (Variables|/Game/_Core/_AdriaanNewShit/Player/BP_Player_DI.BP_Player_DI_C|SetCan%20Interact%20with%20Cap _asbp_player_di true)
  (Variables|Default|SetLookat? true)
  (Development|SetHiddeninGame (Variables|Default|GetPress%20E) false false)
  (Default|GetInfofromCap _output_get self))

(event OnComponentEndOverlap(Sphere)
  (params (OverlappedComponent :type Primitive%20Component%20Object%20Reference) (OtherActor :type Actor%20Object%20Reference) (OtherComp :type Primitive%20Component%20Object%20Reference) (OtherBodyIndex :type Integer))
  (bind _asbp_player_di (Utilities|Casting|CastToBP_Player_DI OtherActor))
  (Variables|Default|SetAs%20BP%20Player%20DI _asbp_player_di)
  (Variables|/Game/_Core/_AdriaanNewShit/Player/BP_Player_DI.BP_Player_DI_C|SetCan%20Interact%20with%20Cap _asbp_player_di false)
  (Variables|Default|SetLookat? false)
  (Development|SetHiddeninGame (Variables|Default|GetPress%20E) true false))

(event EventTick
  (params (DeltaSeconds :type Float%20%28single-precision%29))
  (if (Variables|Default|GetLookat?)
    (Transformation|SetWorldRotation (Variables|Default|GetDefaultSceneRoot) (Math|Rotator|MakeRotator 0.0 0.0 (.yaw (CallFunction|LookatFunction (Variables|Default|GetCaptain) (Variables|/Script/Engine.Character|GetCapsuleComponent (Variables|Default|GetAs%20BP%20Player%20DI))))) false false)
    (Transformation|SetWorldRotation (Variables|Default|GetPress%20E) (Math|Rotator|MakeRotator 0.0 0.0 (.yaw (CallFunction|LookatFunction (Variables|Default|GetPress%20E) (Variables|/Game/_Core/_AdriaanNewShit/Player/BP_Player_DI.BP_Player_DI_C|GetCineCamera%20TEMP (Variables|Default|GetAs%20BP%20Player%20DI))))) false false)))

(event EventStartCamS
  (params (Temp :type Boolean))
  (bind _newcamera_posistion (Variables|Default|GetNewCamera%20Posistion))
  (Default|StartNewCameraPos (Variables|Default|GetAs%20BP%20Player%20DI) (Transformation|GetWorldLocation _newcamera_posistion) (Transformation|GetWorldRotation _newcamera_posistion)))

(fn ConstructionScript)

(fn LookatFunction
  (params (Target%20Start :type Scene%20Component%20Object%20Reference) (Target :type Scene%20Component%20Object%20Reference))
  (return (Math|Rotator|FindLookatRotation (Transformation|GetWorldLocation Target%20Start) (Transformation|GetWorldLocation Target))))