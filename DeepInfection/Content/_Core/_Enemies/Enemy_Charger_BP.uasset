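; Charger enemy Blueprint that takes damage, deals damage through its attack volume and dies with an animation before delayed destruction.
; On BeginPlay it registers itself with its Charger controller, whose CanCharge flag turns off while the player overlaps the detection volume and back on when they leave.
; Hits reduce Health, spawn blood Niagara and print Health for debugging.
; The skin spawn event is empty, and the random material swap is unconnected.
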(event OnComponentBeginOverlap(HeatAttack)
  (params (OverlappedComponent :type Primitive%20Component%20Object%20Reference) (OtherActor :type Actor%20Object%20Reference) (OtherComp :type Primitive%20Component%20Object%20Reference) (OtherBodyIndex :type Integer) (bFromSweep :type Boolean) (SweepResult :type Hit%20Result%20Structure%20%28by%20ref%29))
  (Class|BPIPlayer|GetDMG(Message) OtherActor (Variables|Default|GetEnnemyDMG)))

(event OnComponentBeginOverlap(Playerdetaction)
  (params (OverlappedComponent :type Primitive%20Component%20Object%20Reference) (OtherActor :type Actor%20Object%20Reference) (OtherComp :type Primitive%20Component%20Object%20Reference) (OtherBodyIndex :type Integer) (bFromSweep :type Boolean) (SweepResult :type Hit%20Result%20Structure%20%28by%20ref%29))
  (Utilities|Casting|CastToDI_Player OtherActor)
  (Variables|/Game/_Core/_Enemies/_AiSystems/_Brain/Enemy_CTR_Charger.Enemy_CTR_Charger_C|Setcan%20charge? (Variables|Default|GetAs%20Enemy%20CTR%20Charger) false))

(event OnComponentEndOverlap(Playerdetaction)
  (params (OverlappedComponent :type Primitive%20Component%20Object%20Reference) (OtherActor :type Actor%20Object%20Reference) (OtherComp :type Primitive%20Component%20Object%20Reference) (OtherBodyIndex :type Integer))
  (Utilities|Casting|CastToDI_Player OtherActor)
  (Variables|/Game/_Core/_Enemies/_AiSystems/_Brain/Enemy_CTR_Charger.Enemy_CTR_Charger_C|Setcan%20charge? (Variables|Default|GetAs%20Enemy%20CTR%20Charger) true))

(event Custom|Kill%20Enemy
  (params (Damage :type Float%20%28double-precision%29))
  (if (<= (Variables|Default|GetHealth) 0.001)
    (Components|Animation|PlayAnimation (Variables|Character|GetMesh) "/Game/_Core/_Enemies/_Charger/Enemy_Charger_Anim_Death.Enemy_Charger_Anim_Death" false)
    (Utilities|FlowControl|Delay 7.0)
    (Actor|DestroyActor)))

(event Custom|Spawn%20With%20Dif%20Skinn)

(event EventBeginPlay
  (bind _asenemy_ctr_charger (Utilities|Casting|CastToEnemy_CTR_Charger (Pawn|GetController)))
  (Variables|Default|SetAs%20Enemy%20CTR%20Charger _asenemy_ctr_charger)
  (Default|GettingOwnerChar _asenemy_ctr_charger self))

(event Game|Damage|EventAnyDamage
  (params (Damage :type Float%20%28single-precision%29) (DamageType :type Damage%20Type%20Object%20Reference) (InstigatedBy :type Controller%20Object%20Reference) (DamageCauser :type Actor%20Object%20Reference))
  (bind _output_get (Variables|Default|SetHealth (- (Variables|Default|GetHealth) Damage)))
  (CallFunction|SpawnNiagraEmiter (Variables|Collision|GetCapsuleComponent) "/Game/_PlaceHolderts/Particles/Blood_Niagara.Blood_Niagara")
  (CallFunction|KillEnemy _output_get)
  (Development|PrintString (Utilities|String|ToString(Float) _output_get)))

(fn ConstructionScript)