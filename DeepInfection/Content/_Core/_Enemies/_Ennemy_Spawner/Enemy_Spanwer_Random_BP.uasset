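; Enemy spawner actor that creates a batch of random enemies across its spawn points when play begins.
; On BeginPlay it gathers its eight spawn location components into an array, then starts spawning after a short delay.
; A DoN node looped back through a Delay staggers SpawnAmmount spawns, each picking a random class from Ennemy and a random point's world transform, so points can repeat.
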(event Custom|Spawn%20ennemy%20On%20Location
  (Utilities|FlowControl|DoN (Variables|Default|GetSpawn%20Ammount) :!label _label
    (:Exit
      (Game|SpawnActorfromClass (.OutItem (Utilities|Array|Random (Variables|Default|GetEnnemy))) (Transformation|GetWorldTransform (.OutItem (Utilities|Array|Random (Variables|Default|GetSpawn%20Location%20ARRAY)))) "Undefined" "MultiplyWithRoot" 0 0)
      (Utilities|FlowControl|Delay 0.2)
      (goto _label))))

(event EventBeginPlay
  (CallFunction|SetSpawntoArray)
  (Utilities|FlowControl|Delay 0.2)
  (CallFunction|SpawnEnnemyonLocation))

(event Collision|EventActorBeginOverlap
  (params (OtherActor :type Actor%20Object%20Reference)))

(event EventTick
  (params (DeltaSeconds :type Float%20%28single-precision%29)))

(fn ConstructionScript)

(fn SetSpawntoArray
  (Utilities|Array|Add (Variables|Default|GetSpawn%20Location%20ARRAY) (Variables|Default|GetSpawnLocation7))
  (Utilities|Array|Add (Variables|Default|GetSpawn%20Location%20ARRAY) (Variables|Default|GetSpawnLocation6))
  (Utilities|Array|Add (Variables|Default|GetSpawn%20Location%20ARRAY) (Variables|Default|GetSpawnLocation5))
  (Utilities|Array|Add (Variables|Default|GetSpawn%20Location%20ARRAY) (Variables|Default|GetSpawnLocation4))
  (Utilities|Array|Add (Variables|Default|GetSpawn%20Location%20ARRAY) (Variables|Default|GetSpawnLocation3))
  (Utilities|Array|Add (Variables|Default|GetSpawn%20Location%20ARRAY) (Variables|Default|GetSpawnLocation2))
  (Utilities|Array|Add (Variables|Default|GetSpawn%20Location%20ARRAY) (Variables|Default|GetSpawnLocation1))
  (Utilities|Array|Add (Variables|Default|GetSpawn%20Location%20ARRAY) (Variables|Default|GetSpawnLocation)))