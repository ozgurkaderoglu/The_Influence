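; Enemy spawner actor that places one randomly chosen enemy once the game has begun.
; From BeginPlay it polls a game-begun flag on a short delay loop, then triggers spawning once and destroys its preview component.
; After a configurable delay, it assigns a random class to a child actor component.
; It then messages the first actor found of that class, not necessarily the new one, passing itself.
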(event Custom|Spawn%20ennemy%20On%20Location
  (Utilities|FlowControl|Delay (Variables|Default|GetSpawn%20Timer%20When%20Active))
  (bind _output_get (Variables|Default|SetEnnemyspawnd (.OutItem (Utilities|Array|Random (Variables|Default|GetEnnemy)))))
  (ChildActorComponent|SetChildActorClass (Variables|Default|GetEnnemy1) _output_get)
  (bind _returnvalue (Actor|GetActorOfClass (Variables|Default|GetEnnemyspawnd)))
  (Class|BPIGetDamage|SentInfofromSpawnertoKronone(Message) _returnvalue self))

(event Custom|Start%20Spawning
  (if (Variables|Default|GetDit%20Game%20Begin?) :!label _label
    (Utilities|FlowControl|DoOnce false
      (:Completed
        (CallFunction|SpawnEnnemyonLocation)
        (Components|DestroyComponent (Variables|Default|GetPrevieuwen))))
    (else
      (Utilities|FlowControl|Delay 0.2)
      (goto _label))))

(event EventBeginPlay
  (CallFunction|StartSpawning))

(event Collision|EventActorBeginOverlap
  (params (OtherActor :type Actor%20Object%20Reference)))

(event EventTick
  (params (DeltaSeconds :type Float%20%28single-precision%29)))

(fn ConstructionScript)

(fn OnRepMonstersAlive)