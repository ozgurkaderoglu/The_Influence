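; BP_KronenFast is a Kronen enemy that takes damage and dies.
; On BeginPlay it applies a random material from Textures to its mesh and flags itself as Kronnen on its Enemy_CTR_Main AI controller.
; AnyDamage lowers Health, spawns blood Niagara at the capsule, runs the kill check and prints Health for debugging.
; When Health is depleted, KillEnemy plays a death animation and destroys the actor after a delay.
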(event Custom|Kill%20Enemy
  (params (Damage :type Float%20%28double-precision%29))
  (if (<= (Variables|Default|GetHealth) 0.001)
    (Components|Animation|PlayAnimation (Variables|Character|GetMesh) "/Game/_Core/_Enemies/Kronen_Male/Kronen_Animations_Death1.Kronen_Animations_Death1" false)
    (Utilities|FlowControl|Delay 7.0)
    (Actor|DestroyActor)))

(event Custom|Spawn%20With%20Dif%20Skinn
  (Rendering|Material|SetMaterial (Variables|Character|GetMesh) 0 (.OutItem (Utilities|Array|Random (Variables|Default|GetTextures)))))

(event EventBeginPlay
  (CallFunction|SpawnwithDifSkinn)
  (bind _asenemy_ctr_main (Utilities|Casting|CastToEnemy_CTR_Main (AI|GetAIController self)))
  (Default|GetInfoAI _asenemy_ctr_main true false false false false))

(event Game|Damage|EventAnyDamage
  (params (Damage :type Float%20%28single-precision%29) (DamageType :type Damage%20Type%20Object%20Reference) (InstigatedBy :type Controller%20Object%20Reference) (DamageCauser :type Actor%20Object%20Reference))
  (bind _output_get (Variables|Default|SetHealth (- (Variables|Default|GetHealth) Damage)))
  (CallFunction|SpawnNiagraEmiter (Variables|Collision|GetCapsuleComponent) "/Game/_PlaceHolderts/Particles/Blood_Niagara.Blood_Niagara")
  (CallFunction|KillEnemy _output_get)
  (Development|PrintString (Utilities|String|ToString(Float) _output_get)))

(fn ConstructionScript)