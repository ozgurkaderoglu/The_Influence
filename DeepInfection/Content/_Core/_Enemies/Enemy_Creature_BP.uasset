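; Boss creature enemy that takes damage and drives the player's boss health menu.
; On BeginPlay it stores max health and flags itself as a boss on its Enemy_CTR_Main AI controller.
; End overlaps on the zone component cache the player and alternate showing and hiding the menu through a FlipFlop.
; Damage updates that menu and spawns blood Niagara, but the death check is empty, with animation and destroy nodes unwired.
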(event OnComponentEndOverlap(Enter/ExitBossZone)
  (params (OverlappedComponent :type Primitive%20Component%20Object%20Reference) (OtherActor :type Actor%20Object%20Reference) (OtherComp :type Primitive%20Component%20Object%20Reference) (OtherBodyIndex :type Integer))
  (bind _asdi_player (Utilities|Casting|CastToDI_Player OtherActor))
  (Variables|Default|SetAs%20DI%20Player _asdi_player)
  (Variables|/Game/_Core/_Player/_Widgets/_Widgets/WGP_BossHealthBarr.WGP_BossHealthBarr_C|SetMainBossMax (Variables|/Game/_Core/_Player/DI_Player.DI_Player_C|GetWGP_BossMenu _asdi_player) (Variables|Default|GetMax%20Health%20))
  (Variables|/Game/_Core/_Player/_Widgets/_Widgets/WGP_BossHealthBarr.WGP_BossHealthBarr_C|SetMainBosMin (Variables|/Game/_Core/_Player/DI_Player.DI_Player_C|GetWGP_BossMenu _asdi_player) (Variables|Default|GetHealth))
  (Utilities|FlowControl|FlipFlop
    (:A
      (Default|EnteringBossZone (Variables|/Game/_Core/_Player/DI_Player.DI_Player_C|GetWGP_BossMenu _asdi_player) (Variables|Default|GetHealth) false false true))
    (:B
      (Default|ExetingBossZone (Variables|/Game/_Core/_Player/DI_Player.DI_Player_C|GetWGP_BossMenu _asdi_player)))))

(event Custom|Kill%20Enemy
  (params (Damage :type Float%20%28double-precision%29))
  (if (<= (Variables|Default|GetHealth) 0.001)
    _))

(event EventGettingDamage
  (params (Damage :type Float%20%28double-precision%29))
  (bind _output_get (Variables|Default|SetHealth (- (Variables|Default|GetHealth) Damage)))
  (Variables|/Game/_Core/_Player/_Widgets/_Widgets/WGP_BossHealthBarr.WGP_BossHealthBarr_C|SetMainBosMin (Variables|/Game/_Core/_Player/DI_Player.DI_Player_C|GetWGP_BossMenu (Variables|Default|GetAs%20DI%20Player)) (Variables|Default|GetHealth))
  (CallFunction|SpawnNiagraEmiter (Variables|Collision|GetCapsuleComponent) "/Game/_PlaceHolderts/Particles/Blood_Niagara.Blood_Niagara")
  (CallFunction|KillEnemy _output_get)
  (Development|PrintString (Utilities|String|ToString(Float) _output_get)))

(event EventBeginPlay
  (Variables|Default|SetMax%20Health%20 (Variables|Default|GetHealth))
  (bind _asenemy_ctr_main (Utilities|Casting|CastToEnemy_CTR_Main (AI|GetAIController self)))
  (Default|GetInfoAI _asenemy_ctr_main false false false false true false false))

(fn ConstructionScript)