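; BP_SlidingDoor is a sliding door that opens and closes through its OpenDoor event.
; A sphere overlap sets a flag allowing OpenDoor to run, which also triggers PlayAnims on the DI_Player actor.
; A FlipFlop alternates playing and reversing a timeline that lerps the door's world location between the StartAnim and EndAnim components.
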(event OnComponentBeginOverlap(Sphere)
  (params (OverlappedComponent :type Primitive%20Component%20Object%20Reference) (OtherActor :type Actor%20Object%20Reference) (OtherComp :type Primitive%20Component%20Object%20Reference) (OtherBodyIndex :type Integer) (bFromSweep :type Boolean) (SweepResult :type Hit%20Result%20Structure%20%28by%20ref%29))
  (Variables|Default|SetCan%20do%20lEVVER true))

(event OnComponentEndOverlap(Sphere)
  (params (OverlappedComponent :type Primitive%20Component%20Object%20Reference) (OtherActor :type Actor%20Object%20Reference) (OtherComp :type Primitive%20Component%20Object%20Reference) (OtherBodyIndex :type Integer))
  (Variables|Default|SetCan%20do%20lEVVER false))

(event Custom|OpenDoor
  (if (Variables|Default|GetCan%20do%20lEVVER)
    (bind _returnvalue (Actor|GetActorOfClass "/Game/_Core/_Player/DI_Player.DI_Player_C"))
    (Default|PlayAnims _returnvalue)
    (Utilities|FlowControl|FlipFlop
      (:A
        (bind _newtrack_0 (Timeline|Anim%20door PlayFromStart)
          (:Update
            (Transformation|SetWorldLocation (Variables|Default|GetDoor) (Math|Vector|Lerp(Vector) (Transformation|GetWorldLocation (Variables|Default|GetStart%20Anim)) (Transformation|GetWorldLocation (Variables|Default|GetEnd%20Anim)) _newtrack_0) false false))))
      (:B
        (Timeline|Anim%20door ReverseFromEnd)))))

(event EventBeginPlay)

(event Collision|EventActorBeginOverlap
  (params (OtherActor :type Actor%20Object%20Reference)))

(event EventTick
  (params (DeltaSeconds :type Float%20%28single-precision%29)))

(fn ConstructionScript)