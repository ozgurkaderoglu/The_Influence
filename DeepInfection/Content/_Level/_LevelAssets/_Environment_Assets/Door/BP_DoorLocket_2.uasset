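; BP_DoorLocket_2 is a locked door that swings open and closed when interacted with using the "key2" item.
; The INTERACTOBJ event prints the received item name and, on a match, a FlipFlop alternates a Timeline forward and reverse, with forward updates driving the yaw of the Ankerpoint component.
; SetDoorTokeyInfo writes the door's KeyName into the Key variable of the IF_Character actor found in the level.
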(event Custom|SetDoorTokeyInfo
  (bind _returnvalue (Actor|GetActorOfClass "/Game/_Core/_Player/IF_Character.IF_Character_C"))
  (Variables|/Game/_Core/_Player/IF_Character.IF_Character_C|SetKey _returnvalue (Variables|Default|GetKeyName)))

(event EventINTERACTOBJ
  (params (Interacted%20Actor :type Actor%20Object%20Reference) (ItemName :type Name :default "None"))
  (Development|PrintString (Utilities|String|ToString(Name) ItemName))
  (if (== ItemName "key2")
    (Utilities|FlowControl|FlipFlop
      (:A
        (bind _newtrack_1 (Timeline|Timeline Play)
          (:Update
            (Transformation|SetRelativeRotation (Variables|Default|GetAnkerpoint) (Math|Rotator|MakeRotator 0.0 0.0 _newtrack_1) false false))))
      (:B
        (Timeline|Timeline Reverse)))))

(fn ConstructionScript)