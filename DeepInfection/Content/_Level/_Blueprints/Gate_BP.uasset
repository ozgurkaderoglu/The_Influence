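; Gate actor that slides its GateDoor1 component open and back when StartGate or ReturnGate is called.
; A Timeline track interpolates the door's relative X between the StaticPos and MoveToPos components, keeping StaticPos's Y and Z.
; StartGate plays the Timeline from the start and ReturnGate reverses it from the end.
; An IsGateNotInUse flag ignores calls during movement and resets when the Timeline finishes.
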(event Custom|StartGate
  (bind _staticpos (Variables|Default|GetStaticPos))
  (bind _relativelocation (Variables|/Script/Engine.SceneComponent|GetRelativeLocation _staticpos))
  (if (Variables|Default|GetIsGateNotInUse?)
    (Variables|Default|SetIsGateNotInUse? false)
    (bind _newtrack_0 (Timeline|Timeline PlayFromStart)
      (:Update
        (Transformation|SetRelativeLocation (Variables|Default|GetGate_Door1) (Math|Vector|MakeVector (Math|Float|Lerp (.x _relativelocation) (.x (Variables|/Script/Engine.SceneComponent|GetRelativeLocation (Variables|Default|GetMoveToPos))) _newtrack_0) (.y _relativelocation) (.z _relativelocation)) false false))
      (:Finished
        (Variables|Default|SetIsGateNotInUse? true)))))

(event Custom|ReturnGate
  (bind _staticpos (Variables|Default|GetStaticPos))
  (bind _relativelocation (Variables|/Script/Engine.SceneComponent|GetRelativeLocation _staticpos))
  (if (Variables|Default|GetIsGateNotInUse?)
    (Variables|Default|SetIsGateNotInUse? false)
    (bind _newtrack_0 (Timeline|Timeline ReverseFromEnd)
      (:Update
        (Transformation|SetRelativeLocation (Variables|Default|GetGate_Door1) (Math|Vector|MakeVector (Math|Float|Lerp (.x _relativelocation) (.x (Variables|/Script/Engine.SceneComponent|GetRelativeLocation (Variables|Default|GetMoveToPos))) _newtrack_0) (.y _relativelocation) (.z _relativelocation)) false false))
      (:Finished
        (Variables|Default|SetIsGateNotInUse? true)))))

(event EventBeginPlay)

(event Collision|EventActorBeginOverlap
  (params (OtherActor :type Actor%20Object%20Reference)))

(event EventTick
  (params (DeltaSeconds :type Float%20%28single-precision%29)))

(fn ConstructionScript)