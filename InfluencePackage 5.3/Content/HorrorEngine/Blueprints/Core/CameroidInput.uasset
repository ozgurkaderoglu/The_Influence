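; Input-handling Blueprint for the Cameroid camera that takes over controls from the player while it is in use.
; Use disables player input and enables its own, forwarding turn and look axes to the player pawn.
; The Use action takes a photo, AlternativeUse toggles the flash, and the Cameroid action unequips the camera and restores normal player input.
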(event EventUse
  (params (HorrorEvent :type Boolean))
  (CallFunction|PlayerInput false)
  (CallFunction|ControllerInput true))

(event Input|ActionEvents|InputAction[HE]AlternativeUse
  (params (Key :type Key%20Structure :default "None"))
  (:Pressed
    (bind _asmaster (CallFunction|GetPlayer))
    (Variables|/Game/HorrorEngine/HorrorEngine.HorrorEngine_C|SetCameroidFlashOn _asmaster (not (Variables|/Game/HorrorEngine/HorrorEngine.HorrorEngine_C|GetCameroidFlashOn _asmaster)))))

(event Input|ActionEvents|InputAction[HE]Use
  (params (Key :type Key%20Structure :default "None"))
  (:Pressed
    (bind _asmaster (CallFunction|GetPlayer))
    (Default|TakePhoto _asmaster)))

(event Input|ActionEvents|InputAction[HE]Cameroid
  (params (Key :type Key%20Structure :default "None"))
  (:Pressed
    (bind _asmaster (CallFunction|GetPlayer))
    (Default|UnequipCameroid _asmaster)
    (CallFunction|ControllerInput false)
    (CallFunction|PlayerInput true)))

(event Input|AxisEvents|InputAxis[HE]Turn
  (params (AxisValue :type Float%20%28single-precision%29))
  (Pawn|Input|AddControllerYawInput (Game|Player|GetPlayerPawn 0) AxisValue))

(event Input|AxisEvents|InputAxis[HE]LookUp
  (params (AxisValue :type Float%20%28single-precision%29))
  (Pawn|Input|AddControllerPitchInput (Game|Player|GetPlayerPawn 0) AxisValue))

(fn ConstructionScript)