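; Save data object that holds the player's progress: position, health, key and weapon slots, healing items, ammo and colored keys.
; The SaveAllData event copies every passed-in value into its matching variable, and LoadGame returns all of them at once.
; It only stores and hands back values; no slot writing or disk access happens in this Blueprint.
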(event Custom|SaveAllData
  (params (PlayerPos :type Transform) (Player%20Health :type Float%20%28double-precision%29) (Value%20Keyslot%201 :type Name) (Value%20Keyslot%202 :type Name) (Value%20Keyslot%203 :type Name) (Value%20Rifle%20Slot :type Boolean) (Value%20Shotgun%20Slot :type Boolean) (Value%20Spear%20Gun%20Slot :type Boolean) (Value%20Axe%20Weapon%20Slot :type Boolean) (Value%20Knive%20Slot :type Boolean) (Test%203thitme%20Ammount :type Integer) (Test%20Inv%20Medkit%20Amount :type Integer) (Test%20Inv%20Bandage%20Ammount :type Integer) (TotalAmmoAr :type Integer) (InClipAR :type Integer) (TotalAmmoSG :type Integer) (InClipSG :type Integer) (TotalAmmoHG :type Integer) (InClupHG :type Integer) (Green%20Key :type Boolean) (Red%20Key :type Boolean))
  (Variables|Default|SetPlayerPos PlayerPos)
  (Variables|Default|SetPlayer%20Health Player%20Health)
  (Variables|Default|SetValue%20Keyslot%201 Value%20Keyslot%201)
  (Variables|Default|SetValue%20Keyslot%202 Value%20Keyslot%202)
  (Variables|Default|SetValue%20Keyslot%203 Value%20Keyslot%203)
  (Variables|Default|SetValue%20Rifle%20Slot Value%20Rifle%20Slot)
  (Variables|Default|SetValue%20Shotgun%20Slot Value%20Shotgun%20Slot)
  (Variables|Default|SetValue%20Spear%20Gun%20Slot Value%20Spear%20Gun%20Slot)
  (Variables|Default|SetValue%20Axe%20Weapon%20Slot Value%20Axe%20Weapon%20Slot)
  (Variables|Default|SetValue%20Knive%20Slot Value%20Knive%20Slot)
  (Variables|Default|SetTest%203thitme%20Ammount Test%203thitme%20Ammount)
  (Variables|Default|SetTest%20Inv%20Medkit%20Amount Test%20Inv%20Medkit%20Amount)
  (Variables|Default|SetTest%20Inv%20Bandage%20Ammount Test%20Inv%20Bandage%20Ammount)
  (Variables|Default|SetTotalAmmoAr TotalAmmoAr)
  (Variables|Default|SetInClipAR InClipAR)
  (Variables|Default|SetTotalAmmoSG TotalAmmoSG)
  (Variables|Default|SetInClipSG InClipSG)
  (Variables|Default|SetTotalAmmoHG TotalAmmoHG)
  (Variables|Default|SetInClupHG InClupHG)
  (Variables|Default|SetGreen%20Key Green%20Key)
  (Variables|Default|SetRed%20Key Red%20Key))

(fn LoadGame
  (return (Variables|Default|GetPlayerPos) (Variables|Default|GetPlayer%20Health) (Variables|Default|GetValue%20Keyslot%201) (Variables|Default|GetValue%20Keyslot%202) (Variables|Default|GetValue%20Keyslot%203) (Variables|Default|GetValue%20Rifle%20Slot) (Variables|Default|GetValue%20Shotgun%20Slot) (Variables|Default|GetValue%20Spear%20Gun%20Slot) (Variables|Default|GetValue%20Axe%20Weapon%20Slot) (Variables|Default|GetValue%20Knive%20Slot) (Variables|Default|GetTest%203thitme%20Ammount) (Variables|Default|GetTest%20Inv%20Medkit%20Amount) (Variables|Default|GetTest%20Inv%20Bandage%20Ammount) (Variables|Default|GetTotalAmmoAr) (Variables|Default|GetInClipAR) (Variables|Default|GetTotalAmmoSG) (Variables|Default|GetInClipSG) (Variables|Default|GetTotalAmmoHG) (Variables|Default|GetInClupHG) (Variables|Default|GetGreen%20Key) (Variables|Default|GetRed%20Key)))