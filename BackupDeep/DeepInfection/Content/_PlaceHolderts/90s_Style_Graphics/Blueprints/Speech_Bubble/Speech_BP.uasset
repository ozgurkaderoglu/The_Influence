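; Speech bubble actor that displays configurable text on a plane in the world.
; Set_Text, noted as called from a speech macro, applies the user-set text, color, scales, height offset and visibility, and gives the plane a dynamic material instance.
; Tick billboards the text by copying the player camera rotation, then flipping it 180 degrees in yaw.
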(event Custom|Set_Text
  (bind _plane (Variables|Default|GetPlane))
  (bind _textrender (Variables|Default|GetTextRender))
  (bind _plane_2 (Variables|Default|GetPlane))
  (bind _returnvalue (Transformation|GetWorldScale _plane_2))
  ;[1 1 1] An event that is called in the speech macro to apply all user defined settings.
  (Rendering|Components|TextRender|SetText _textrender (Variables|Default|GetSpeech_Text))
  (Rendering|Components|TextRender|SetTextRenderColor _textrender (Variables|Default|GetText_Color))
  (Transformation|SetWorldScale3D _plane_2 (Math|Vector|MakeVector (.x _returnvalue) (.y _returnvalue) (Variables|Default|GetBubble_Scale)))
  (Transformation|SetActorScale3D (Math|Conversions|ToVector(Float) (Variables|Default|GetWhole_Scale)))
  (Transformation|AddWorldOffset (Variables|Default|GetPlane) (Math|Vector|MakeVector 0.0 0.0 (Variables|Default|GetHeight_Offset)) false false)
  (bind _returnvalue_2 (Rendering|Material|CreateDynamicMaterialInstance _plane 0 (Variables|Default|GetSpeech_Bubble_Mat) "None" :!class /Script/Engine.PrimitiveComponent))
  (Rendering|Material|SetMaterial _plane 0 _returnvalue_2)
  (Development|SetHiddeninGame _plane (Variables|Default|GetHide_Bubble?) false))

(event EventTick
  (params (DeltaSeconds :type Float%20%28single-precision%29))
  (bind _textrender (Variables|Default|GetTextRender))
  ;[1 1 1] Setting text to face the camera direction
  (Transformation|SetWorldRotation _textrender (.Rotation (Math|Transform|BreakTransform (Transformation|GetActorTransform (Game|GetPlayerCameraManager 0)))) false false)
  (Transformation|AddLocalRotation _textrender "0,-180.000000, 0" false false))

(fn ConstructionScript)