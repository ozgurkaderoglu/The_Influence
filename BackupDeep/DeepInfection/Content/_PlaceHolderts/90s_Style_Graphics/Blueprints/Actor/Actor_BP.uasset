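; Actor_BP is a pawn with animated blinking and speech-driven mouth movement, and it spawns its default controller on BeginPlay.
; A self-restarting retriggerable delay triggers brief blinks at random intervals by toggling a custom primitive data float on the mesh.
; The Speech_Voice audio envelope, scaled by VoiceSensitivity, drives a second primitive data float for speech, which Stop_Mouth resets to zero.
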(event OnAudioMultiEnvelopeValue(Speech_Voice)
  (params (AverageEnvelopeValue :type Float%20%28single-precision%29) (MaxEnvelope :type Float%20%28single-precision%29) (NumWaveInstances :type Integer))
  ;[1 1 1] Enable Speech Movement
  (bind _output_get (Variables|Default|SetSpeech_Amount (* AverageEnvelopeValue (Variables|Default|GetVoice_Sensitivity))))
  (Rendering|Material|SetCustomPrimitiveDataFloat (Variables|Character|GetMesh) 31 _output_get))

(event Custom|Stop_Mouth
  ;[1 1 1] Enable Speech Movement
  (bind _output_get (Variables|Default|SetSpeech_Amount 0.0))
  (Rendering|Material|SetCustomPrimitiveDataFloat (Variables|Character|GetMesh) 31 _output_get))

(event Custom|Blink
  (bind _mesh (Variables|Character|GetMesh))
  ;[1 1 1] Blinking
  (Utilities|FlowControl|Sequence :!label _label
    (:then_0
      (Utilities|FlowControl|RetriggerableDelay (Math|Random|RandomFloatinRange 1.0 3.0))
      (goto _label))
    (:then_1
      (bind _output_get (Variables|Default|SetBlink_Value 1.0))
      (Rendering|Material|SetCustomPrimitiveDataFloat _mesh 30 _output_get)
      (Utilities|FlowControl|Delay 0.2)
      (bind _output_get_2 (Variables|Default|SetBlink_Value 0.0))
      (Rendering|Material|SetCustomPrimitiveDataFloat _mesh 30 _output_get_2))))

(event EventBeginPlay
  ;[1 1 1] BeginPlay
  ;[1 1 1] Spawn default controller for this Pawn, and get possessed by it.
  (Pawn|SpawnDefaultController)
  ;[1 1 1] Calling blink event
  (CallFunction|Blink))

(fn ConstructionScript)