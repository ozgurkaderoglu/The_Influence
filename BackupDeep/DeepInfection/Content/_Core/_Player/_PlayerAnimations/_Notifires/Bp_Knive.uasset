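; Animation notify that resolves the player's melee hit for axe, knife or neither weapon in DI_Player's animations.
; It sphere-traces a short distance ahead of the player, with debug drawing left on.
; Axe and knife hits send damage, higher for the axe, and play a stab sound and blood Niagara effect at the player's mesh.
; With neither weapon active, a hit only destroys wood_BP actors.
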(fn ReceivedNotify
  (params (MeshComp :type Skeletal%20Mesh%20Component%20Object%20Reference) (Animation :type Anim%20Sequence%20Base%20Object%20Reference) (EventReference :type Anim%20Notify%20Event%20Reference%20Structure%20%28by%20ref%29))
  (bind _returnvalue (Components|GetOwner MeshComp))
  (bind _returnvalue_2 (Transformation|GetActorLocation _returnvalue))
  (bind _asdi_player (Utilities|Casting|CastToDI_Player _returnvalue))
  (bind (_outhit _returnvalue_3) (Collision|SphereTraceByChannel _returnvalue_2 (+ _returnvalue_2 (* (Transformation|GetActorForwardVector _returnvalue) 1e+02)) 2e+01 "TraceTypeQuery3" false 0 "ForDuration"))
  (if _returnvalue_3
    (if (Variables|/Game/_Core/_Player/DI_Player.DI_Player_C|GetHolding%20axe _asdi_player)
      (Class|BPIGetDamage|GettingDamage(Message) (.HitActor (Collision|BreakHitResult _outhit)) 1e+02)
      (Audio|PlaySoundatLocation "/Game/_Core/Item_sounds/Knife_Stab.Knife_Stab" (Transformation|GetWorldLocation (Variables|/Script/Engine.Character|GetMesh _asdi_player)) "0, 0, 0" 1.0 1.0 0.0 0 0 0 0)
      (Niagara|SpawnSystematLocation "/Game/_PlaceHolderts/Particles/Blood_Niagara.Blood_Niagara" (Transformation|GetWorldLocation (Variables|/Script/Engine.Character|GetMesh _asdi_player)) :!label _label)
      (elif (Variables|/Game/_Core/_Player/DI_Player.DI_Player_C|GetKnive%20Active? _asdi_player)
        (Class|BPIGetDamage|GettingDamage(Message) (.HitActor (Collision|BreakHitResult _outhit)) 7e+01)
        (Audio|PlaySoundatLocation "/Game/_Core/Item_sounds/Knife_Stab.Knife_Stab" (Transformation|GetWorldLocation (Variables|/Script/Engine.Character|GetMesh _asdi_player)) "0, 0, 0" 1.0 1.0 0.0 0 0 0 0)
        (goto _label)
        (else
          (bind _aswood_bp (Utilities|Casting|CastTowood_BP (.HitActor (Collision|BreakHitResult _outhit))))
          (Default|DestroyActorFunction _aswood_bp))))))