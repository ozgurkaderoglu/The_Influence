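; Female Kronen enemy that spawns with a random skin material and identifies itself as female to its Enemy_CTR_Main AI controller.
; Damage lowers health and spawns blood Niagara effects.
; At zero health it plays a death animation, asks its stored spawner to spawn another enemy, and disables movement and collision.
; Death also notifies the controller, may drop a random item, and destroys the actor after a delay.
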(event Custom|Kill%20Enemy
  (params (Damage :type Float%20%28double-precision%29))
  (if (<= (Variables|Default|GetHealth) 0.001)
    (Components|Animation|PlayAnimation (Variables|Character|GetMesh) "/Game/_Core/_Enemies/Kronen_Female/KronenFemale_Animations_Death1.KronenFemale_Animations_Death1" false)
    (bind _asennemy_spawner (Utilities|Casting|CastToEnnemySpawner (Variables|Default|GetSpawner))
      (:then
        (Default|SpawnEnnemyonLocation _asennemy_spawner))
      (:CastFailed
        _))
    (Utilities|FlowControl|Sequence
      (:then_0
        (Pawn|Components|CharacterMovement|DisableMovement (Variables|Character|GetCharacterMovement))
        (CallFunction|DropItem?)
        (Utilities|FlowControl|Sequence
          (:then_0
            (Utilities|FlowControl|Delay 7.0)
            (Actor|DestroyActor))
          (:then_1
            (bind _asenemy_ctr_main (Utilities|Casting|CastToEnemy_CTR_Main (AI|GetAIController self)))
            (Default|EnnemyIsDeath _asenemy_ctr_main))))
      (:then_1
        (Collision|SetCollisionEnabled (Variables|Collision|GetCapsuleComponent) "NoCollision")))))

(event Custom|Spawn%20With%20Dif%20Skinn
  (Rendering|Material|SetMaterial (Variables|Character|GetMesh) 0 (.OutItem (Utilities|Array|Random (Variables|Default|GetTextures)))))

(event Custom|Drop%20Item?
  (Variables|Default|SetRandom (Math|Random|RandomIntegerinRange 1 5))
  (if (== (Variables|Default|GetRandom) 2)
    (Game|SpawnActorfromClass (.OutItem (Utilities|Array|Random (Variables|Default|GetItems%20To%20Drop))) (Math|Transform|MakeTransform (Transformation|GetActorLocation) "0, 0, 0" "1.000000,1.000000,1.000000") "Undefined" "MultiplyWithRoot" 0 0)))

(event EventGettingDamage
  (params (Damage :type Float%20%28double-precision%29))
  (bind _output_get (Variables|Default|SetHealth (- (Variables|Default|GetHealth) Damage)))
  (CallFunction|SpawnNiagraEmiter (Variables|Collision|GetCapsuleComponent) "/Game/_PlaceHolderts/Particles/Blood_Niagara.Blood_Niagara")
  (CallFunction|KillEnemy _output_get)
  (Development|PrintString (Utilities|String|ToString(Float) _output_get)))

(event EventBeginPlay
  (CallFunction|SpawnwithDifSkinn)
  (bind _asenemy_ctr_main (Utilities|Casting|CastToEnemy_CTR_Main (AI|GetAIController self)))
  (Default|GetInfoAI _asenemy_ctr_main false false false false false true false))

(event EventSentInfofromSpawnertoKronone
  (params (Spawner :type Actor%20Object%20Reference))
  (Variables|Default|SetSpawner Spawner))

(fn ConstructionScript)