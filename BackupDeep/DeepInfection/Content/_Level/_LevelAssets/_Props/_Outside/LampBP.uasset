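; Outdoor lamp prop that flickers its spotlight and light-beam component when IsHorrorMode is set at BeginPlay.
; HorrorMode calls itself through Delays, using a DoN counter against a re-rolled random limit to blink both components off and on in short bursts.
; When a burst ends, Rest resets the counter and the lamp stays lit through random pauses before the next burst.
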(event Custom|Horror%20Mode
  (if (Variables|Default|GetIs%20Vis?)
    (bind _output_get (Variables|Default|SetRandomNub (Math|Random|RandomIntegerinRange 2 6)))
    (Utilities|FlowControl|Delay 0.2)
    (bind _counter (Utilities|FlowControl|DoN _output_get)
      (:Exit
        (Variables|Default|SetCounter _counter)
        (if (>= (Variables|Default|GetCounter) (Variables|Default|GetRandomNub))
          (Variables|Default|SetIs%20Vis? false)
          (CallFunction|Rest)
          (Utilities|FlowControl|Delay (Math|Random|RandomFloatinRange 0.5 3.0) :!label _label)
          (CallFunction|HorrorMode)
          (else
            ;[1 1 1] Not vis
            (Rendering|SetVisibility (Variables|Default|GetSpotLight) false false)
            (Rendering|SetVisibility (Variables|Default|GetS_EV_SimpleLightBeam_03) false false)
            (Utilities|FlowControl|Delay 0.2)
            (Rendering|SetVisibility (Variables|Default|GetSpotLight) true false)
            (Rendering|SetVisibility (Variables|Default|GetS_EV_SimpleLightBeam_03) true false)
            (CallFunction|HorrorMode)))))
    (else
      ;[1 1 1] Vis
      (Rendering|SetVisibility (Variables|Default|GetSpotLight) true false)
      (Rendering|SetVisibility (Variables|Default|GetS_EV_SimpleLightBeam_03) true false)
      (Variables|Default|SetIs%20Vis? true)
      (goto _label))))

(event Custom|Rest
  (Variables|Default|SetCounter 0)
  (Utilities|FlowControl|DoN (stale Custom|Horror%20Mode _output_get)) ; enters at Reset
)

(event EventBeginPlay
  (if (Variables|Default|Getis%20horrorMode?)
    (CallFunction|HorrorMode)))

(event Collision|EventActorBeginOverlap
  (params (OtherActor :type Actor%20Object%20Reference)))

(event EventTick
  (params (DeltaSeconds :type Float%20%28single-precision%29)))

(fn ConstructionScript)