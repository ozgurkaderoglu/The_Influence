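; Fixed-camera zone that switches the view to a referenced camera while the player is inside its bounds, in the style of classic fixed-angle games.
; Each tick it tests the capsule location against the bounds, using DoOnce latches to toggle the overlap state.
; While active, the camera can rotate to track the player, and exiting can restore the player's camera.
; It also mirrors the player camera's aspect constraint at 4:3.
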(event Custom|Follow_Player
  (bind _camera_ref (Variables|Default|GetCamera_Ref))
  ;[1 1 1] Camera will follow player if can follow is checked
  (if (Variables|Default|GetCam_Follow?)
    (if (Variables|Default|GetOverlapping%20?)
      (Transformation|SetActorRotation _camera_ref (Math|Rotator|FindLookatRotation (Transformation|GetActorLocation _camera_ref) (+ (Transformation|GetActorLocation (Game|GetPlayerCharacter 0)) (Variables|Default|GetLook_At_Offset)))))))

(event Custom|Set_Camera
  (bind _returnvalue (Game|GetPlayerCharacter 0))
  (bind _returnvalue_2 (Game|GetPlayerController 0))
  ;[1 1 1] Setting Camera
  (if (not (Variables|Default|GetDisable_Cam?))
    (Utilities|IsValid (Variables|Default|GetCamera_Ref)
      (:Is%20Valid
        (if (Variables|Default|GetOverlapping%20?)
          (Utilities|FlowControl|Sequence
            (:then_0
              (Game|Player|SetViewTargetwithBlend _returnvalue_2 (Variables|Default|GetCamera_Ref) 0.0 "VTBlend_Linear" 0.0 false)
              (CallFunction|FollowPlayer))
            (:then_1
              (goto _label Reset)))
          (else
            ;;[1 1 1] Restoring Default player, camera if checked
            (if (Variables|Default|GetReset_Default_Cam_On_End?)
              (Utilities|FlowControl|DoOnce false :!label _label
                (:Completed
                  (Game|Player|SetViewTargetwithBlend _returnvalue_2 _returnvalue 0.0 "VTBlend_Linear" 0.0 false)
                  (Default|ResetCamera (.AsPlayer%20Character%20BP (Utilities|Casting|CastToPlayer_Character_BP _returnvalue))))))))))))

(event Custom|Check_Aspect_Ratio
  (bind _camera_ref (Variables|Default|GetCamera_Ref))
  (bind _cameracomponent (Variables|/Script/Engine.CameraActor|GetCameraComponent _camera_ref))
  ;[1 1 1] Checking aspect ratio changes to adjust fixed camera aspect ration
  (if (Variables|/Script/Engine.CameraComponent|GetbConstrainAspectRatio (Variables|/Game/90s_Style_Graphics/Blueprints/Player/Player_Character_BP.Player_Character_BP_C|GetFollowCamera (.AsPlayer%20Character%20BP (Utilities|Casting|CastToPlayer_Character_BP (Game|GetPlayerCharacter 0)))))
    (Utilities|FlowControl|DoOnce false :!label _label
      (:Completed
        (Variables|/Script/Engine.CameraComponent|SetAspectRatio _cameracomponent 1.333333)
        (Class|CameraComponent|SetConstraintAspectRatio _cameracomponent true)
        (goto _label_2 Reset)))
    (else
      (Utilities|FlowControl|DoOnce false :!label _label_2
        (:Completed
          (Class|CameraComponent|SetConstraintAspectRatio _cameracomponent false)
          (goto _label Reset))))))

(event Custom|In_Bounds_Check
  (bind _returnvalue (Game|GetPlayerCharacter 0))
  (bind _overlapping_bounds (Variables|Default|GetOverlapping_Bounds))
  (bind (_origin _boxextent) (Collision|GetComponentBounds _overlapping_bounds))
  (bind _capsulecomponent (Variables|/Script/Engine.Character|GetCapsuleComponent _returnvalue))
  (bind _returnvalue_2 (Transformation|GetWorldLocation _capsulecomponent))
  (bind _returnvalue_3 (- _origin _boxextent))
  (bind _returnvalue_4 (+ _origin _boxextent))
  (bind (_x _y _z) (Math|Vector|BreakVector _returnvalue_4))
  (bind (_x_2 _y_2 _z_2) (Math|Vector|BreakVector _returnvalue_3))
  (bind (_x_3 _y_3 _z_3) (Math|Vector|BreakVector _returnvalue_2))
  ;[1 1 1] In Bounds Checker
  (if (Math|Boolean|ANDBoolean (<= _x_3 _x) (<= _y_3 _y) (<= _z_3 _z) (not (>= _x_2 _x_3)) (not (>= _y_2 _y_3)) (not (>= _z_2 _z_3)))
    (Utilities|FlowControl|Sequence
      (:then_0
        (Utilities|FlowControl|DoOnce false :!label _label
          (:Completed
            (Variables|Default|SetOverlapping%20? true)
            (Variables|Default|SetActivated_Cam true))))
      (:then_1
        (goto _label_2 Reset)))
    (else
      (Utilities|FlowControl|Sequence
        (:then_0
          (Utilities|FlowControl|DoOnce false :!label _label_2
            (:Completed
              (Variables|Default|SetOverlapping%20? false)
              (Variables|Default|SetActivated_Cam false))))
        (:then_1
          (goto _label Reset))))))

(event EventTick
  (params (DeltaSeconds :type Float%20%28single-precision%29))
  ;[1 1 1] Checkers
  (CallFunction|InBoundsCheck)
  (CallFunction|SetCamera)
  (CallFunction|CheckAspectRatio))

(fn ConstructionScript)